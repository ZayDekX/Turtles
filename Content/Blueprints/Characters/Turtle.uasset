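; Turtle character that is driven by a behavior tree and destroys itself on reaching its target.
; Init stores the target and nest, copies them and move/wait timings into the blackboard, and binds the AI's move-completed event, which triggers destruction near the target.
; RunAI starts the tree separately.
; Spawn and destruction play sound and particle effects, while a timeline plays footsteps at a rate scaled by velocity.
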(event Custom|Run%20AI
  (AI|RunBehaviorTree (AI|GetAIController self) "/Game/Blueprints/AI/TurtleBehavior.TurtleBehavior"))

(event Custom|Init
  (params (Target%20Point :type Actor%20Object%20Reference) (Nest :type Nest%20Object%20Reference))
  (Variables|Default|SetTarget Target%20Point)
  (Variables|Default|SetNest Nest)
  (CallFunction|BindBlackboardData)
  (|BindeventstoanAI))

(event EventDestroyed
  (Audio|PlaySoundatLocation "/Game/Sounds/Windows_XP_Balloon.Windows_XP_Balloon" (Transformation|GetActorLocation) "0, 0, 0" 1e+01 1.0 0.0 0 0 0)
  (Effects|SpawnEmitteratLocation "/Game/FXVarietyPack/Particles/P_ky_waterBallHit.P_ky_waterBallHit" (Transformation|GetActorLocation)))

(event EventBeginPlay
  (Audio|PlaySoundatLocation "/Game/Sounds/Windows_XP_Balloon.Windows_XP_Balloon" (Transformation|GetActorLocation) "0, 0, 0" 1e+01 0.8 0.0 0 0 0)
  (Effects|SpawnEmitteratLocation "/Game/FXVarietyPack/Particles/P_ky_explosion.P_ky_explosion" (Transformation|GetActorLocation))
  (Components|Timeline|SetPlayRate (Variables|Default|GetFootsteps%20Timeline) 0.0)
  (Timeline|Footsteps%20Timeline Play
    (:Step
      (Audio|PlaySoundatLocation "/Game/Sounds/Steps.Steps" (Transformation|GetActorLocation) "0, 0, 0" 1.0 1.0 0.0 0 0 0))))

(event EventTick
  (params (DeltaSeconds :type Float%20%28single-precision%29))
  (Components|Timeline|SetPlayRate (Variables|Default|GetFootsteps%20Timeline) (/ (Math|Vector|VectorLength (Transformation|GetVelocity)) 5e+02)))

(fn ConstructionScript)

(fn BindBlackboardData
  (Utilities|FlowControl|Sequence
    (:then_0
      (bind _blackboardcomponent (Class|AIController|UseBlackboard (AI|GetAIController self) "/Game/Blueprints/AI/TurtleBlackboard.TurtleBlackboard"))
      (LocalVariables|SetBlackboard%20component _blackboardcomponent))
    (:then_1
      (AI|Components|Blackboard|SetValueasObject (LocalVariables|GetBlackboard%20component) (Utilities|String|StringToName "Target") (Variables|Default|GetTarget))
      (AI|Components|Blackboard|SetValueasObject (LocalVariables|GetBlackboard%20component) (Utilities|String|StringToName "Nest") (Variables|Default|GetNest))
      (AI|Components|Blackboard|SetValueasFloat (LocalVariables|GetBlackboard%20component) (Utilities|String|StringToName "MoveForwardTime") (Variables|Default|GetMoveForwardTime))
      (AI|Components|Blackboard|SetValueasFloat (LocalVariables|GetBlackboard%20component) (Utilities|String|StringToName "MoveBackwardTime") (Variables|Default|GetMoveBackwardTime))
      (AI|Components|Blackboard|SetValueasFloat (LocalVariables|GetBlackboard%20component) (Utilities|String|StringToName "WaitingTime") (Variables|Default|GetWaitingTime)))))

(event Custom|OnMoveCompleted
  (params (RequestID :type AI%20Request%20ID%20Structure) (Result :type EPathFollowingResult%20Enum :default "Success"))
  (switch Utilities|FlowControl|Switch|SwitchonEPathFollowingResult Result
    (:Success
      (if (< (Math|Vector|VectorLength (- (Transformation|GetActorLocation (Variables|Default|GetTarget)) (Transformation|GetActorLocation))) 5e+01)
        (Actor|DestroyActor)))))