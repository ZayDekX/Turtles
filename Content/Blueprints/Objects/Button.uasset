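; Button is an interactable object that spawns a turtle from its linked Nest and starts that turtle's AI.
; A cooldown starts at ActivationDelay on construction and counts down each Tick, blocking Interact until it runs out.
; A successful spawn resets the cooldown and plays a quiet, high-pitched piston sound at the button's location.
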(event EventTick
  (params (DeltaSeconds :type Float%20%28single-precision%29))
  (CallFunction|UpdateDelay DeltaSeconds))

(fn ConstructionScript
  (Variables|Default|SetTime%20To%20Activation (Variables|Default|GetActivation%20Delay)))

(fn Interact
  (if (<= (Variables|Default|GetTime%20To%20Activation) 0.0)
    (bind _turtle (Default|SpawnTurtle (Variables|Default|GetNest)))
    (Utilities|IsValid _turtle
      (:Is%20Valid
        (Default|RunAI _turtle)
        (Variables|Default|SetTime%20To%20Activation (Variables|Default|GetActivation%20Delay))
        (Audio|PlaySoundatLocation "/Game/Sounds/Piston_extend.Piston_extend" (Transformation|GetActorLocation) "0, 0, 0" 0.05 5.0 0.0 0 0 0)))))

(fn UpdateDelay
  (params (Delta%20Seconds :type Float%20%28single-precision%29))
  (if (> (Variables|Default|GetTime%20To%20Activation) 0.0)
    (Variables|Default|SetTime%20To%20Activation (- (Variables|Default|GetTime%20To%20Activation) Delta%20Seconds))))